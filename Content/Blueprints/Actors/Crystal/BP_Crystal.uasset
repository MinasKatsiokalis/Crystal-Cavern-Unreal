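; Collectible crystal actor that spins in place until the player overlaps it, then flies into the player and vanishes.
; Tick adds a fixed yaw step each frame, so spin speed follows frame rate.
; A player overlap stores starting values and plays a timeline whose tracks lerp location toward the pawn's live position, scale to zero and point light intensity toward zero.
; The actor destroys itself when the timeline finishes.
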(event EventTick
  (params (DeltaSeconds :type Float%20%28single-precision%29))
  ;[1 1 1] Crystal Rotation
  (CallFunction|RotateCrystal))

(event Collision|EventActorBeginOverlap
  (params (OtherActor :type Actor%20Object%20Reference))
  ;[1 1 1] Destroy when Collected
  (Utilities|IsPlayer OtherActor
    (:IsPlayer
      ;[1 1 1] Move to Player Animation
      (CallFunction|StoreStartingValues)
      (bind (_direction _smooth_lerp_alpha _scale_transition _light_intensity) (Timeline|Alpha%20Blend%20Timeline Play)
        (:Update
          (CallFunction|MovetoPlayer _smooth_lerp_alpha)
          (CallFunction|CrystalScale _scale_transition)
          (CallFunction|AdjustLight _light_intensity))
        (:Finished
          (Actor|DestroyActor))))))

(fn ConstructionScript)

(fn MovetoPlayer
  (params (Alpha :type Float%20%28single-precision%29))
  (Transformation|SetActorLocation (Math|Vector|Lerp(Vector) (Variables|Default|GetLerpStartLocation) (Transformation|GetActorLocation (Game|Player|GetPlayerPawn 0)) Alpha) false false))

(fn StoreStartingValues
  (Variables|Default|SetLerpStartLocation (Transformation|GetActorLocation))
  (Variables|Default|SetStartScale (Transformation|GetActorScale3D))
  (Variables|Default|SetIntensity (Variables|/Script/Engine.LightComponentBase|GetIntensity (Variables|Default|GetPointLight))))

(fn CrystalScale
  (params (Alpha :type Float%20%28single-precision%29))
  (Transformation|SetActorScale3D (Math|Vector|Lerp(Vector) (Variables|Default|GetStartScale) "0, 0, 0" Alpha)))

(fn AdjustLight
  (params (Alpha :type Float%20%28single-precision%29))
  (Rendering|Components|Light|SetIntensity (Variables|Default|GetPointLight) (Math|Float|Lerp (Variables|Default|GetLightIntensity) 0.0 Alpha)))

(fn RotateCrystal
  (Transformation|SetActorRotation (Math|Rotator|MakeRotator 0.0 0.0 (+ (.yaw (Transformation|GetActorRotation)) 1.0))))