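; BP_Cannon is a cannon actor that automatically and repeatedly fires ball projectiles from BeginPlay onward.
; After a FireRate delay, SpawnProjectile emits an explosion particle and spawns a BP_Projectile at the Arrow's location and rotation, each with its own scale variable.
; A timeline then animates the barrel's recoil along local Y, and its Cannon Fired event restarts the delay to form the firing loop.
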(event EventBeginPlay
  ;[0.276 0.276 0.276] Based on FireRate spawn/fire a projectile
  (Utilities|FlowControl|Delay (Variables|CannonProperties|GetFire%20Rate) :!label _label)
  (CallFunction|SpawnProjectile)
  ;;[0.3802 0.1703 0.1703] Fire Animation by moving Cannon Barel backwards
  (bind _cannon_barel_location (Timeline|Cannon%20Fire%20Timeline PlayFromStart)
    (:Update
      (Transformation|SetRelativeLocation (Variables|Default|GetCannon%20Barel%20) (Math|Vector|MakeVector 0.0 _cannon_barel_location 0.0) false false))
    (:Cannon%20Fired
      (goto _label))))

(fn ConstructionScript)

(fn SpawnProjectile
  (bind _arrow (Variables|Default|GetArrow))
  (bind _returnvalue (Transformation|GetWorldLocation _arrow))
  (bind _returnvalue_2 (Transformation|GetWorldRotation _arrow))
  ;[1 1 1] Spawns a Ball projectile and Emits an Explosiotn praticle at Arrow location
  (Effects|SpawnEmitteratLocation "/Game/StarterContent/Particles/P_Explosion.P_Explosion" _returnvalue _returnvalue_2 (Math|Conversions|ToVector(Float) (Variables|CannonProperties|GetExplosion%20Scale)))
  (Game|SpawnActorfromClass "/Game/Blueprints/Actors/Projectiles/BP_Projectile.BP_Projectile_C" (Math|Transform|MakeTransform _returnvalue _returnvalue_2 (Math|Conversions|ToVector(Float) (Variables|CannonProperties|GetProjectile%20Scale))) "AlwaysSpawn" 0 0))