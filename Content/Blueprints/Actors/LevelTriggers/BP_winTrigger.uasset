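; BP_winTrigger is a level trigger that ends a level when the player overlaps it with no BP_Crystal actors left in the world.
; If any crystals remain, it prints a warning instead.
; On completion it finds the current level in a LevelNames array and opens the next entry by name.
; On the last entry it prints a game-finished message rather than loading a level.
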(event Collision|EventActorBeginOverlap
  (params (OtherActor :type Actor%20Object%20Reference))
  (Utilities|IsPlayer OtherActor
    (:IsPlayer
      (if (CallFunction|AnyCrystalsRemaining)
        (Development|PrintString "YOU HAVE NOT COLLECTED ALL THE CRYSTALS!" true true "(R=0.038050,G=0.920322,B=1.000000,A=1.000000)" 3.0)
        (else
          (CallFunction|CompleteLevel))))))

(fn ConstructionScript)

(fn AnyCrystalsRemaining
  (bind _outactors (Actor|GetAllActorsOfClass "/Game/Blueprints/Actors/Crystal/BP_Crystal.BP_Crystal_C"))
  (return (> (Utilities|Array|Length _outactors) 0)))

(fn GetCurrentLevelIndex
  (bind _returnvalue (Game|GetCurrentLevelName true))
  (return (Utilities|Array|FindItem (Variables|Default|GetlevelNames) (Utilities|String|StringToName _returnvalue))))

(fn CompleteLevel
  (if (CallFunction|IstheFinalLevel)
    (Development|PrintString "CONGRATZ! YOU FINISHED THE GAME!" true true "(R=0.000000,G=1.000000,B=0.025283,A=1.000000)" 5.0)
    (else
      (CallFunction|LoadNextLevel))))

(fn IstheFinalLevel
  (return (== (Utilities|Array|LastIndex (Variables|Default|GetlevelNames)) (CallFunction|GetCurrentLevelIndex))))

(fn LoadNextLevel
  (Game|OpenLevel(byName) (CallFunction|GetNextLevelName)))

(fn GetNextLevelName
  (return (Utilities|Array|Get(acopy) (Variables|Default|GetlevelNames) (+ (CallFunction|GetCurrentLevelIndex) 1))))