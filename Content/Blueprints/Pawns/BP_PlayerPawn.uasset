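; Player pawn for a rolling ball that is moved by torque and restarts the level when it takes damage.
; Both movement axes feed the same torque call, which applies the axis value to X and Y together on the static mesh.
; The camera fades in at start; any damage triggers a one-shot fade-out, delay and level reload.
; R reloads the level immediately and Escape quits the game.
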(event EventBeginPlay
  ;[1 1 1] Fade In Camera
  (CallFunction|FadeinCamera 1.5))

(event Game|Damage|EventAnyDamage
  (params (Damage :type Float%20%28single-precision%29) (DamageType :type Damage%20Type%20Object%20Reference) (InstigatedBy :type Controller%20Object%20Reference) (DamageCauser :type Actor%20Object%20Reference))
  ;[1 1 1] Restart After Killed
  (Utilities|ReloadAfterDie 0.5))

(event Input|AxisEvents|InputAxisMoveForwards/Backwards
  (params (AxisValue :type Float%20%28single-precision%29))
  (bind _torqueforce_ (Variables|Default|GettorqueForce%20))
  ;[1 1 1] Ball Movement
  (Class|PrimitiveComponent|AddTorqueinRadians (Variables|Default|GetStaticMesh) (Math|Vector|MakeVector (* (stale Input|AxisEvents|InputAxisMoveRight/Left AxisValue) _torqueforce_) (* AxisValue _torqueforce_) 0.0) "None" true))

(event Input|AxisEvents|InputAxisMoveRight/Left
  (params (AxisValue :type Float%20%28single-precision%29))
  (bind _torqueforce_ (Variables|Default|GettorqueForce%20))
  ;[1 1 1] Ball Movement
  (Class|PrimitiveComponent|AddTorqueinRadians (Variables|Default|GetStaticMesh) (Math|Vector|MakeVector (* AxisValue _torqueforce_) (* (stale Input|AxisEvents|InputAxisMoveForwards/Backwards AxisValue) _torqueforce_) 0.0) "None" true))

(event Input|KeyboardEvents|R
  (params (Key :type Key%20Structure :default "None"))
  ;[1 1 1] Restart Level
  (:Released
    (bind _returnvalue (Game|GetCurrentLevelName true))
    (Game|OpenLevel(byName) (Utilities|String|StringToName _returnvalue))))

(event Input|KeyboardEvents|Escape
  (params (Key :type Key%20Structure :default "None"))
  ;[1 1 1] Quit Game
  (:Released
    (Game|QuitGame 0 "Quit" false)))

(fn ConstructionScript)

(fn FadeinCamera
  (params (Duration :type Float%20%28single-precision%29))
  (CameraFades|StartCameraFade (Game|GetPlayerCameraManager 0) 1.0 0.0 Duration "(R=0.000000,G=0.000000,B=0.000000,A=1.000000)" false false))

(fn FadeOutCamera
  (params (Duration :type Float%20%28single-precision%29))
  (CameraFades|StartCameraFade (Game|GetPlayerCameraManager 0) 0.0 1.0 Duration "(R=0.000000,G=0.000000,B=0.000000,A=1.000000)" false true))

(fn RealoadScene
  (bind _returnvalue (Game|GetCurrentLevelName true))
  (Game|OpenLevel(byName) (Utilities|String|StringToName _returnvalue)))